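; Base character Blueprint for an NPC that wanders, idles and sleeps at random.
; Shortly after possession, LookForState randomly picks Walk, Idle or Sleep, each playing a looping animation directly on the mesh.
; Walk uses AIMoveTo to a random reachable nearby point, falling back to Idle on failure.
; Successful moves and randomly timed Idle or Sleep delays return to LookForState, forming an event-driven state loop without Tick.
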(event `Look For State`
  (switch `int` (`KismetMathLibrary.RandomIntegerInRange` 0 2)
    (:`0`
      (`self.Walk`))
    (:`1`
      (`self.Idle`))
    (:`2`
      (`self.Sleep`))))

(event `self.ReceivePossessed`
  (params (NewController :type "Controller Object Reference"))
  (if (not false)
    (`KismetSystemLibrary.Delay` 2.0)
    (`self.Look For State`)))

(event `Walk`
  (bind _mesh (`self.Mesh`))
  (`SkeletalMeshComponent.PlayAnimation` _mesh "/Game/Standard_Walk_mixamo_com.Standard_Walk_mixamo_com" true)
  (`|AIMoveTo` self (`NavigationSystemV1.K2_GetRandomReachablePointInRadius` (`SceneComponent.K2_GetComponentLocation` _mesh) 3000.0 null null) null
    (:`OnSuccess`
      (`self.Look For State`))
    (:`OnFail`
      (`self.Idle`))))

(event `Idle`
  (`SkeletalMeshComponent.PlayAnimation` (`self.Mesh`) "/Game/Idle_Anim_mixamo_com.Idle_Anim_mixamo_com" true)
  (`KismetSystemLibrary.Delay` (`KismetMathLibrary.RandomFloatInRange` 0.0 20.0))
  (`self.Look For State`))

(event `Sleep`
  (`SkeletalMeshComponent.PlayAnimation` (`self.Mesh`) "/Game/Sleeping_Idle_mixamo_com.Sleeping_Idle_mixamo_com" true)
  (`KismetSystemLibrary.Delay` (`KismetMathLibrary.RandomFloatInRange` 0.0 20.0))
  (`self.Look For State`))

(fn `UserConstructionScript`)